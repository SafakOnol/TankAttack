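; Game mode Blueprint for Tank Attack that puts the match's start, in-game and end screens on the viewport.
; StartGame shows the start widget, then adds the in-game widget after a fixed delay, without removing the first here.
; GameWon shows the end widget and sets its text to a win or loss message from the WonGame flag.
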(event EventBeginPlay)

(event EventTick
  (params (DeltaSeconds :type Float%20%28single-precision%29)))

(event EventStartGame
  ;[1 1 1] Start Game Screen
  (bind _returnvalue (UserInterface|CreateWidget "/Game/Blueprints/Widgets/WBP_StartGameWidget.WBP_StartGameWidget_C"))
  (UserInterface|Viewport|AddtoViewport _returnvalue 0)
  ;[1 1 1] In Game Widget
  (Utilities|FlowControl|Delay 5.0)
  (bind _returnvalue_2 (UserInterface|CreateWidget "/Game/Blueprints/Widgets/WBP_InGameWidget.WBP_InGameWidget_C"))
  (UserInterface|Viewport|AddtoViewport _returnvalue_2 0))

(event EventGameWon
  (params (bWonGame :type Boolean))
  ;[1 1 1] End Game Screen
  (bind _returnvalue (UserInterface|CreateWidget "/Game/Blueprints/Widgets/WBP_EndGameWidget.WBP_EndGameWidget_C"))
  (UserInterface|Viewport|AddtoViewport _returnvalue 0)
  (Rendering|Components|TextRender|SetText (Variables|/Game/Blueprints/Widgets/WBP_EndGameWidget.WBP_EndGameWidget_C|GetDisplayText _returnvalue) (select bWonGame "YOU WON!" "YOU LOST!")))

(fn ConstructionScript)